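; Wizard player character that casts mana shot, fireball, freeze and ultimate nova spells, and adds a crosshair on BeginPlay.
; BeginPlay also applies the saved cosmetic mesh from DT_Cosmetics.
; Light attack fires directly with a one-second DoOnce lockout, while F/G/H skills play montages and start cooldowns.
; Separate spawn events launch projectiles from the hand socket along camera rotation, or place the nova via camera line trace.
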(event `self.ReceiveBeginPlay`
  (`parent.ReceiveBeginPlay`)
  (bind _returnvalue (`|CreateWidget` "/Game/UI/Archer_Crosshair/W_Crosshair.W_Crosshair_C"))
  (`UserWidget.AddToViewport` _returnvalue 0)
  (bind _asmy_game_instance (cast `/Game/UI/MyGameInstance` (`GameplayStatics.GetGameInstance`)))
  (bind _returnvalue_2 (`|GetDataTableRow` "/Game/Structures/DT_Cosmetics.DT_Cosmetics" (`/Game/UI/SG_PlayerProfile.EquippedCosmetic_RowName` (`/Game/UI/MyGameInstance.CurrentSave` _asmy_game_instance)))
    (:`then`
      (`SkeletalMeshComponent.SetSkeletalMeshAsset` (`self.Mesh`) (`.MeshToLoad_7_81A7C0874C972DBFBF80A5AB94619375` (break `/Game/Structures/Struct_Cosmetic` _returnvalue_2))))))

(event `SpawnFireball`
  (`|SpawnActorFromClass` "/Game/Blueprints/Characters/BP_Fireball.BP_Fireball_C" (`KismetMathLibrary.MakeTransform` (`SceneComponent.GetSocketLocation` (`self.Mesh`) "castspell_r") (`PlayerCameraManager.GetCameraRotation` (`GameplayStatics.GetPlayerCameraManager` 0))) "Undefined" "MultiplyWithRoot" null self))

(event `EnhancedInput|/Game/Inputs/InputActions/IA_LightAttack`
  (params (ActionValue :type Boolean) (ElapsedSeconds :type "Float (double-precision)") (TriggeredSeconds :type "Float (double-precision)") (InputAction :type "InputAction Object Reference" :default "/Game/Inputs/InputActions/IA_LightAttack.IA_LightAttack"))
  (:`Started`
    (`/Engine/EditorBlueprintResources/StandardMacros.DoOnce` false :!label _label
      (:`Completed`
        (`|SpawnActorFromClass` "/Game/Blueprints/Characters/BP_ManaShot.BP_ManaShot_C" (`KismetMathLibrary.MakeTransform` (`SceneComponent.GetSocketLocation` (`self.Mesh`) "castspell_r") (`PlayerCameraManager.GetCameraRotation` (`GameplayStatics.GetPlayerCameraManager` 0))) "Undefined" "MultiplyWithRoot" null self)
        (`KismetSystemLibrary.Delay` 1.0)
        (goto _label :!via `Reset`)))))

(event `SpawnFreeze`
  (`|SpawnActorFromClass` "/Game/Blueprints/Characters/BP_FreezeShot.BP_FreezeShot_C" (`KismetMathLibrary.MakeTransform` (`SceneComponent.GetSocketLocation` (`self.Mesh`) "castspell_r") (`PlayerCameraManager.GetCameraRotation` (`GameplayStatics.GetPlayerCameraManager` 0))) "Undefined" "MultiplyWithRoot" null self))

(event `EnhancedInput|/Game/Inputs/InputActions/IA_Skill_F`
  (params (ActionValue :type Boolean) (ElapsedSeconds :type "Float (double-precision)") (TriggeredSeconds :type "Float (double-precision)") (InputAction :type "InputAction Object Reference" :default "/Game/Inputs/InputActions/IA_Skill_F.IA_Skill_F"))
  (:`Started`
    (if (`self.CanUse_F?`)
      (`self.PlayAnimMontage` "/Game/Animations/Wizard_Animations/CastFIreball.CastFIreball")
      (`self.Start_Cooldown_F`))))

(event `EnhancedInput|/Game/Inputs/InputActions/IA_Skill_G`
  (params (ActionValue :type Boolean) (ElapsedSeconds :type "Float (double-precision)") (TriggeredSeconds :type "Float (double-precision)") (InputAction :type "InputAction Object Reference" :default "/Game/Inputs/InputActions/IA_Skill_G.IA_Skill_G"))
  (:`Started`
    (if (`self.CanUse_G?`)
      (`self.PlayAnimMontage` "/Game/Animations/Wizard_Animations/CastFreeze.CastFreeze")
      (`self.Start_Cooldown_G`))))

(event `SpawnUltimateNova`
  (bind _returnvalue (`GameplayStatics.GetPlayerCameraManager` 0))
  (bind _returnvalue_2 (`PlayerCameraManager.GetCameraLocation` _returnvalue))
  (bind _outhit (`KismetSystemLibrary.LineTraceSingle` _returnvalue_2 (+ _returnvalue_2 (* (`KismetMathLibrary.GetForwardVector` (`PlayerCameraManager.GetCameraRotation` _returnvalue)) 2000.0)) "TraceTypeQuery1"))
  (`|SpawnActorFromClass` "/Game/Blueprints/Characters/BP_UltimateNova.BP_UltimateNova_C" (`KismetMathLibrary.MakeTransform` (`.Location` (`GameplayStatics.BreakHitResult` _outhit))) "Undefined" "MultiplyWithRoot" null self))

(event `EnhancedInput|/Game/Inputs/InputActions/IA_Skill_H`
  (params (ActionValue :type Boolean) (ElapsedSeconds :type "Float (double-precision)") (TriggeredSeconds :type "Float (double-precision)") (InputAction :type "InputAction Object Reference" :default "/Game/Inputs/InputActions/IA_Skill_H.IA_Skill_H"))
  (:`Started`
    (if (`self.CanUse_H?`)
      (`self.PlayAnimMontage` "/Game/Animations/Wizard_Animations/UltimateNova.UltimateNova")
      (`self.Start_Cooldown_H`))))

(fn `UserConstructionScript`
  (`parent.UserConstructionScript`))