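; Base player character that handles Enhanced Input movement, health and death, two-weapon switching and the pause menu.
; On possession it creates the HUD, which receives health updates through an event dispatcher; zero health disables input and opens the lose menu.
; Number keys swap the weapon mesh, base damage and highlighted slot.
; Timeline-driven cooldown events gate skills F, G and H and fill their HUD bars, without implementing the skills themselves.
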(event `Key|Tab` :paused true
  (params (Key :type "Key Structure"))
  (bind _returnvalue (`GameplayStatics.GetPlayerController` 0))
  (bind _returnvalue_2 (`GameplayStatics.GetPlayerController` 0))
  ; HUD and Connection Logic
  (:`Pressed`
    (if (`GameplayStatics.IsGamePaused`)
      (`Widget.RemoveFromParent` (`self.ActivePauseMenu`))
      (`GameplayStatics.SetGamePaused` false)
      (set `PlayerController.bShowMouseCursor` false _returnvalue_2)
      (`WidgetBlueprintLibrary.SetInputMode_GameOnly` _returnvalue_2)
      (else
        (bind _returnvalue_3 (`|CreateWidget` "/Game/UI/Pause_Menu/WBP_PauseMenu.WBP_PauseMenu_C"))
        (bind _output_get (set `self.ActivePauseMenu` _returnvalue_3))
        (`UserWidget.AddToViewport` _output_get 0)
        (`GameplayStatics.SetGamePaused` true)
        (`WidgetBlueprintLibrary.SetInputMode_GameAndUIEx` _returnvalue _returnvalue_3)
        (set `PlayerController.bShowMouseCursor` true _returnvalue)))))

(event `self.ReceiveBeginPlay`
  (bind _returnvalue (`GameplayStatics.GetPlayerController` 0))
  (bind _returnvalue_2 (pcsubsystem `EnhancedInputLocalPlayerSubsystem` _returnvalue))
  ; HUD and Connection Logic
  (`WidgetBlueprintLibrary.SetInputMode_GameOnly` _returnvalue)
  (set `PlayerController.bShowMouseCursor` false _returnvalue)
  (`/Engine/EditorBlueprintResources/StandardMacros.IsValid` _returnvalue_2
    (:`Is Valid`
      (`EnhancedInputSubsystemInterface.AddMappingContext` _returnvalue_2 "/Game/Inputs/IMC_BaseMapping.IMC_BaseMapping" 0 (struct))
      (`StaticMeshComponent.SetStaticMesh` (`self.EquippedWeapon`) (`self.Weapon1_Mesh`))
      (set `self.CurrentBaseDamage` 25.0)
      (`KismetSystemLibrary.Delay` 0.1)
      (`/Game/UI/HealthBar_HUD/WBP_AbilitySlot.ToggleGlow` (`/Game/UI/HealthBar_HUD/WBP_Hud.Slot_Weapon1` (`self.HUD_Ref`)) true)
      (`/Game/UI/HealthBar_HUD/WBP_AbilitySlot.ToggleGlow` (`/Game/UI/HealthBar_HUD/WBP_Hud.Slot_Weapon2` (`self.HUD_Ref`)) false))))

(event `EnhancedInput|/Game/Inputs/InputActions/IA_Look`
  (params (ActionValue :type "Vector2D Structure") (ElapsedSeconds :type "Float (double-precision)") (TriggeredSeconds :type "Float (double-precision)") (InputAction :type "InputAction Object Reference" :default "/Game/Inputs/InputActions/IA_Look.IA_Look"))
  ; Character Movement
  (:`Triggered`
    (`self.AddControllerYawInput` ActionValue_X)
    (`self.AddControllerPitchInput` ActionValue_Y)))

(event `EnhancedInput|/Game/Inputs/InputActions/IA_MoveFoward`
  (params (ActionValue :type "Float (double-precision)") (ElapsedSeconds :type "Float (double-precision)") (TriggeredSeconds :type "Float (double-precision)") (InputAction :type "InputAction Object Reference" :default "/Game/Inputs/InputActions/IA_MoveFoward.IA_MoveFoward"))
  (bind (_returnvalue_roll _returnvalue_pitch _returnvalue_yaw) (`KismetMathLibrary.BreakRotator` (`self.GetControlRotation`)))
  ; Character Movement
  (:`Triggered`
    (`self.AddMovementInput` (`KismetMathLibrary.GetForwardVector` (`KismetMathLibrary.MakeRotator` 0.0 0.0 _returnvalue_yaw)) ActionValue)))

(event `EnhancedInput|/Game/Inputs/InputActions/IA_MoveRight`
  (params (ActionValue :type "Float (double-precision)") (ElapsedSeconds :type "Float (double-precision)") (TriggeredSeconds :type "Float (double-precision)") (InputAction :type "InputAction Object Reference" :default "/Game/Inputs/InputActions/IA_MoveRight.IA_MoveRight"))
  (bind (_returnvalue_roll _returnvalue_pitch _returnvalue_yaw) (`KismetMathLibrary.BreakRotator` (`self.GetControlRotation`)))
  ; Character Movement
  (:`Triggered`
    (`self.AddMovementInput` (`KismetMathLibrary.GetRightVector` (`KismetMathLibrary.MakeRotator` 0.0 0.0 _returnvalue_yaw)) ActionValue)))

(event `self.ReceiveAnyDamage`
  (params (Damage :type "Float (single-precision)") (DamageType :type "DamageType Object Reference") (InstigatedBy :type "Controller Object Reference") (DamageCauser :type "Actor Object Reference"))
  (bind _returnvalue (`GameplayStatics.GetPlayerController` 0))
  ; Health Logic
  (bind _output_get (set `self.CurrentHealth` (`KismetMathLibrary.FClamp` (- (`self.CurrentHealth`) Damage) 0.0 (`self.MaxHealth`))))
  (`self.E_HealthUpdated` _output_get (`self.MaxHealth`))
  (if (== _output_get 0.0)
    (set `self.IsDead?` true)
    (`SkeletalMeshComponent.PlayAnimation` (`self.Mesh`) "/Game/FreeAnimationLibrary/Animations/UnarmedProne/anim_Prone_Idle.anim_Prone_Idle" false)
    (`self.DisableInput` (`GameplayStatics.GetPlayerController` 0))
    (`KismetSystemLibrary.Delay` 1.5)
    (bind _returnvalue_2 (`|CreateWidget` "/Game/UI/Lose_Menu/WBP_LoseMenu.WBP_LoseMenu_C"))
    (`UserWidget.AddToViewport` _returnvalue_2 0)
    (set `PlayerController.bShowMouseCursor` true _returnvalue)
    (`WidgetBlueprintLibrary.SetInputMode_UIOnlyEx` _returnvalue _returnvalue_2)))

(event `EnhancedInput|/Game/Inputs/InputActions/IA_Sprint`
  (params (ActionValue :type Boolean) (ElapsedSeconds :type "Float (double-precision)") (TriggeredSeconds :type "Float (double-precision)") (InputAction :type "InputAction Object Reference" :default "/Game/Inputs/InputActions/IA_Sprint.IA_Sprint"))
  (bind _charactermovement (`self.CharacterMovement`))
  ; Character Movement
  (:`Triggered`
    (set `CharacterMovementComponent.MaxWalkSpeed` 900.0 _charactermovement))
  (:`Canceled`
    (set `CharacterMovementComponent.MaxWalkSpeed` 400.0 _charactermovement :!label _label))
  (:`Completed`
    (goto _label)))

(event `EnhancedInput|/Game/Inputs/InputActions/IA_Crouch`
  (params (ActionValue :type Boolean) (ElapsedSeconds :type "Float (double-precision)") (TriggeredSeconds :type "Float (double-precision)") (InputAction :type "InputAction Object Reference" :default "/Game/Inputs/InputActions/IA_Crouch.IA_Crouch"))
  ; Character Movement
  (:`Triggered`
    (`self.Crouch`))
  (:`Completed`
    (`self.UnCrouch`)))

(event `self.ReceivePossessed`
  (params (NewController :type "Controller Object Reference"))
  ; Health Logic
  (bind _returnvalue (`|CreateWidget` "/Game/UI/HealthBar_HUD/WBP_Hud.WBP_Hud_C"))
  (bind _output_get (set `self.HUD_Ref` _returnvalue))
  (`UserWidget.AddToViewport` _returnvalue 0)
  (`UserWidget.AddToViewport` _output_get 0)
  (`/Game/UI/HealthBar_HUD/WBP_Hud.Initialize` _returnvalue self)
  (`self.E_HealthUpdated` (`self.CurrentHealth`) (`self.MaxHealth`)))

(event `EnhancedInput|/Game/Inputs/InputActions/IA_Jump`
  (params (ActionValue :type Boolean) (ElapsedSeconds :type "Float (double-precision)") (TriggeredSeconds :type "Float (double-precision)") (InputAction :type "InputAction Object Reference" :default "/Game/Inputs/InputActions/IA_Jump.IA_Jump"))
  ; Character Movement
  (:`Started`
    (if (not (`self.IsJumping?`))
      (`self.Jump`)))
  (:`Canceled`
    (`self.StopJumping` :!label _label_2))
  (:`Completed`
    (goto _label_2)))

(event `Key|One`
  (params (Key :type "Key Structure"))
  (:`Pressed`
    (`/Game/UI/HealthBar_HUD/WBP_AbilitySlot.ToggleGlow` (`/Game/UI/HealthBar_HUD/WBP_Hud.Slot_Weapon1` (`self.HUD_Ref`)) true)
    (`/Game/UI/HealthBar_HUD/WBP_AbilitySlot.ToggleGlow` (`/Game/UI/HealthBar_HUD/WBP_Hud.Slot_Weapon2` (`self.HUD_Ref`)) false)
    (`StaticMeshComponent.SetStaticMesh` (`self.EquippedWeapon`) (`self.Weapon1_Mesh`))
    (set `self.CurrentBaseDamage` 25.0)))

(event `Start_Cooldown_F`
  (if (`self.CanUse_F?`)
    (set `self.CanUse_F?` false)
    (bind (_direction _fillamount) (`Timeline|Cooldown_F_Timer` :!via `PlayFromStart`)
      (:`Update`
        (`ProgressBar.SetPercent` (`/Game/UI/HealthBar_HUD/WBP_AbilitySlot.CooldownBar` (`/Game/UI/HealthBar_HUD/WBP_Hud.Slot_skill_F` (`self.HUD_Ref`))) _fillamount))
      (:`Finished`
        (set `self.CanUse_F?` true)))))

(event `self.OnJumped`
  ; Character Movement
  (set `self.IsJumping?` true))

(event `self.OnLanded`
  (params (Hit :type "HitResult Structure (by ref)"))
  ; Character Movement
  (`KismetSystemLibrary.Delay` 0.8)
  (set `self.IsJumping?` false))

(event `Key|Two`
  (params (Key :type "Key Structure"))
  (:`Pressed`
    (`/Game/UI/HealthBar_HUD/WBP_AbilitySlot.ToggleGlow` (`/Game/UI/HealthBar_HUD/WBP_Hud.Slot_Weapon1` (`self.HUD_Ref`)) false)
    (`/Game/UI/HealthBar_HUD/WBP_AbilitySlot.ToggleGlow` (`/Game/UI/HealthBar_HUD/WBP_Hud.Slot_Weapon2` (`self.HUD_Ref`)) true)
    (`StaticMeshComponent.SetStaticMesh` (`self.EquippedWeapon`) (`self.Weapon2_Mesh`))
    (set `self.CurrentBaseDamage` 15.0)))

(event `Start_Cooldown_G`
  (if (`self.CanUse_G?`)
    (set `self.CanUse_G?` false)
    (bind (_direction _fillamount) (`Timeline|Cooldown_G_Timer` :!via `PlayFromStart`)
      (:`Update`
        (`ProgressBar.SetPercent` (`/Game/UI/HealthBar_HUD/WBP_AbilitySlot.CooldownBar` (`/Game/UI/HealthBar_HUD/WBP_Hud.Slot_Skill_G` (`self.HUD_Ref`))) _fillamount))
      (:`Finished`
        (set `self.CanUse_G?` true)))))

(event `Start_Cooldown_H`
  (if (`self.CanUse_H?`)
    (set `self.CanUse_H?` false)
    (bind (_direction _fillamount) (`Timeline|Cooldown_H_Timer` :!via `PlayFromStart`)
      (:`Update`
        (`ProgressBar.SetPercent` (`/Game/UI/HealthBar_HUD/WBP_AbilitySlot.CooldownBar` (`/Game/UI/HealthBar_HUD/WBP_Hud.Slot_Skill_H` (`self.HUD_Ref`))) _fillamount))
      (:`Finished`
        (set `self.CanUse_H?` true)))))

(fn `UserConstructionScript`)