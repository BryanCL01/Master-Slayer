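; Warrior character Blueprint with light, heavy and combo sword attacks on Enhanced Input actions.
; Each input calls a shared SwordAttack event with its own montage, radius and damage.
; An IsAttacking flag blocks new attacks while the montage plays and clears only on completion.
; Montage notifies trigger a stationary multi-sphere trace at the Sword component, applying damage to every Pawn hit result.
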(event `SwordAttack`
  (params (AttackMontage :type "AnimMontage Object Reference") (AttackRadius :type "Float (double-precision)") (AttackDamage :type "Float (double-precision)"))
  (bind _returnvalue (`SceneComponent.K2_GetComponentLocation` (`self.Sword`)))
  (if (not (`self.IsAttacking?`))
    (`|PlayMontage` (`self.Mesh`) AttackMontage
      (:`then`
        (set `self.IsAttacking?` true))
      (:`OnCompleted`
        (set `self.IsAttacking?` false))
      (:`OnNotifyBegin`
        (bind (_outhits _returnvalue_2) (`KismetSystemLibrary.SphereTraceMultiForObjects` _returnvalue _returnvalue AttackRadius (`|MakeArray` "ObjectTypeQuery3" :!type "EObjectTypeQuery Enum")))
        (if _returnvalue_2
          (for _array_element _outhits
            (`GameplayStatics.ApplyDamage` (`.HitActor` (`GameplayStatics.BreakHitResult` _array_element)) AttackDamage)))))))

(event `EnhancedInput|/Game/Inputs/InputActions/IA_LightAttack`
  (params (ActionValue :type Boolean) (ElapsedSeconds :type "Float (double-precision)") (TriggeredSeconds :type "Float (double-precision)") (InputAction :type "InputAction Object Reference" :default "/Game/Inputs/InputActions/IA_LightAttack.IA_LightAttack"))
  (:`Started`
    (`self.SwordAttack` "/Game/Animations/AM_LightAttack.AM_LightAttack" 50.0 25.0)))

(event `EnhancedInput|/Game/Inputs/InputActions/IA_HeavyAttack`
  (params (ActionValue :type Boolean) (ElapsedSeconds :type "Float (double-precision)") (TriggeredSeconds :type "Float (double-precision)") (InputAction :type "InputAction Object Reference" :default "/Game/Inputs/InputActions/IA_HeavyAttack.IA_HeavyAttack"))
  (:`Started`
    (`self.SwordAttack` "/Game/Animations/AM_HeavyAttack.AM_HeavyAttack" 50.0 50.0)))

(event `EnhancedInput|/Game/Inputs/InputActions/IA_ComboAttack`
  (params (ActionValue :type Boolean) (ElapsedSeconds :type "Float (double-precision)") (TriggeredSeconds :type "Float (double-precision)") (InputAction :type "InputAction Object Reference" :default "/Game/Inputs/InputActions/IA_ComboAttack.IA_ComboAttack"))
  (:`Started`
    (`self.SwordAttack` "/Game/Animations/AM_Combo.AM_Combo" 100.0 25.0)))

(fn `UserConstructionScript`
  (`parent.UserConstructionScript`))