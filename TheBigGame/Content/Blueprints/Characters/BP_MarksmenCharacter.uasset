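; Playable Marksman character with bow aiming, draw-and-release firing and three cooldown-gated skills.
; Bow input, spread shot (G) and arrow rain (H) are delegated to ACBowMechanics, while F spawns a trap at the character's feet.
; Aiming toggles the HUD crosshair and drives a timeline that blends camera FOV and spring-arm offset from values cached at BeginPlay, reversing on release.
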(event `self.ReceiveBeginPlay`
  (`parent.ReceiveBeginPlay`)
  (set `self.InitialFOV` (`CameraComponent.FieldOfView` (`self.Camera`)))
  (set `self.InitialBoomOffset` (`SpringArmComponent.SocketOffset` (`self.SpringArm`))))

(event `EnhancedInput|/Game/Inputs/InputActions/IA_AimBow`
  (params (ActionValue :type Boolean) (ElapsedSeconds :type "Float (double-precision)") (TriggeredSeconds :type "Float (double-precision)") (InputAction :type "InputAction Object Reference" :default "/Game/Inputs/InputActions/IA_AimBow.IA_AimBow"))
  (:`Started`
    (`/Game/Blueprints/Characters/AC_BowMechanics.AimBegin` (`self.AC_BowMechanics`))
    (`self.AimCameraBegin`)
    (`Widget.SetVisibility` (`/Game/UI/HealthBar_HUD/WBP_Hud.CrosshairWidget` (`self.HUD_Ref`)) "Visible"))
  (:`Completed`
    (`/Game/Blueprints/Characters/AC_BowMechanics.AimEnd` (`self.AC_BowMechanics`))
    (`self.AimCameraEnd`)
    (`Widget.SetVisibility` (`/Game/UI/HealthBar_HUD/WBP_Hud.CrosshairWidget` (`self.HUD_Ref`)) "Hidden")))

(event `EnhancedInput|/Game/Inputs/InputActions/IA_Skill_F`
  (params (ActionValue :type Boolean) (ElapsedSeconds :type "Float (double-precision)") (TriggeredSeconds :type "Float (double-precision)") (InputAction :type "InputAction Object Reference" :default "/Game/Inputs/InputActions/IA_Skill_F.IA_Skill_F"))
  (:`Triggered`
    (if (`self.CanUse_F?`)
      (`|SpawnActorFromClass` "/Game/Blueprints/Characters/BP_Trap.BP_Trap_C" (`KismetMathLibrary.MakeTransform` (- (`self.K2_GetActorLocation`) (0.0 0.0 90.0))) "Undefined" "MultiplyWithRoot" null null)
      (`self.Start_Cooldown_F`))))

(event `AimCameraBegin`
  (bind (_direction _aimalpha) (`Timeline|AimCameraTimeline` :!label _label)
    (:`Update`
      (`CameraComponent.SetFieldOfView` (`self.Camera`) (`KismetMathLibrary.Lerp` (`self.InitialFOV`) (`self.AimFOV`) _aimalpha))
      (set `SpringArmComponent.SocketOffset` (`KismetMathLibrary.VLerp` (`self.InitialBoomOffset`) (`self.AimBoomOffset`) _aimalpha) (`self.SpringArm`)))))

(event `EnhancedInput|/Game/Inputs/InputActions/IA_Skill_G`
  (params (ActionValue :type Boolean) (ElapsedSeconds :type "Float (double-precision)") (TriggeredSeconds :type "Float (double-precision)") (InputAction :type "InputAction Object Reference" :default "/Game/Inputs/InputActions/IA_Skill_G.IA_Skill_G"))
  (:`Triggered`
    (if (`self.CanUse_G?`)
      (`/Game/Blueprints/Characters/AC_BowMechanics.FireSpreadShot` (`self.AC_BowMechanics`))
      (`self.Start_Cooldown_G`))))

(event `AimCameraEnd`
  (goto _label :!via `Reverse`))

(event `EnhancedInput|/Game/Inputs/InputActions/IA_Skill_H`
  (params (ActionValue :type Boolean) (ElapsedSeconds :type "Float (double-precision)") (TriggeredSeconds :type "Float (double-precision)") (InputAction :type "InputAction Object Reference" :default "/Game/Inputs/InputActions/IA_Skill_H.IA_Skill_H"))
  (:`Triggered`
    (if (`self.CanUse_H?`)
      (`/Game/Blueprints/Characters/AC_BowMechanics.FireArrowRain` (`self.AC_BowMechanics`))
      (`self.Start_Cooldown_H`))))

(event `EnhancedInput|/Game/Inputs/InputActions/IA_FireBow`
  (params (ActionValue :type Boolean) (ElapsedSeconds :type "Float (double-precision)") (TriggeredSeconds :type "Float (double-precision)") (InputAction :type "InputAction Object Reference" :default "/Game/Inputs/InputActions/IA_FireBow.IA_FireBow"))
  ; Fire Bow
  (:`Started`
    (`/Game/Blueprints/Characters/AC_BowMechanics.DrawBowBegin` (`self.AC_BowMechanics`)))
  (:`Completed`
    (`/Game/Blueprints/Characters/AC_BowMechanics.FireArrowBegin` (`self.AC_BowMechanics`))))

(fn `UserConstructionScript`
  (`parent.UserConstructionScript`))