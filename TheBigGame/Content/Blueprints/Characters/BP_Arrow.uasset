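; Arrow projectile that stays inert until fired, then flies, sticks into what it hits and deals damage scaled by shot strength.
; Fire enables collision and adds a projectile movement component at runtime, with strength blending speed and gravity.
; On overlap it ignores other arrows and its instigator, removes movement and attaches to the closest skeletal bone or the hit component.
; Hits on physics-simulating components also apply an impulse to the arrow's own collision box.
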(event `self.ReceiveBeginPlay`
  (`PrimitiveComponent.SetCollisionEnabled` (`self.CollisionBox`) "NoCollision"))

(event `Fire`
  (params (Direction :type "Vector Structure") (Strength :type "Float (double-precision)"))
  (bind _output_get (set `self.ArrowStrength` Strength))
  (`PrimitiveComponent.SetCollisionEnabled` (`self.CollisionBox`) "QueryAndPhysics")
  (bind _returnvalue (`AddComponent|NODE_AddProjectileMovementComponent-0`))
  (bind _output_get_2 (set `self.ProjectileMovementRef` _returnvalue))
  (set `MovementComponent.Velocity` (* Direction (`KismetMathLibrary.Lerp` (`self.MinSpeed`) (`self.MaxSpeed`) _output_get)) _output_get_2)
  (set `ProjectileMovementComponent.ProjectileGravityScale` (`KismetMathLibrary.Lerp` (`self.MaxGravity`) (`self.MinGravity`) _output_get) _output_get_2))

(event `self.CollisionBox.OnComponentBeginOverlap`
  (params (OverlappedComponent :type "PrimitiveComponent Object Reference") (OtherActor :type "Actor Object Reference") (OtherComp :type "PrimitiveComponent Object Reference") (OtherBodyIndex :type Integer) (bFromSweep :type Boolean) (SweepResult :type "HitResult Structure (by ref)"))
  (bind (_bblockinghit _binitialoverlap _time _distance _location _impactpoint _normal _impactnormal _physmat _hitactor _hitcomponent) (`GameplayStatics.BreakHitResult` SweepResult))
  (bind _returnvalue (`self.GetComponentByClass` _hitactor "/Script/Engine.SkeletalMeshComponent"))
  (cast `/Game/Blueprints/Characters/BP_Arrow` OtherActor
    (:`CastFailed`
      (if (!= OtherActor (`self.GetInstigator`))
        (`/Engine/EditorBlueprintResources/StandardMacros.IsValid` (`self.ProjectileMovementRef`)
          (:`Is Valid`
            (set `self.ImpactVelocity` (`MovementComponent.Velocity` (`self.ProjectileMovementRef`)))
            (if (`SceneComponent.IsSimulatingPhysics` _hitcomponent "None")
              (`PrimitiveComponent.AddImpulse` (`self.CollisionBox`) (`self.ImpactVelocity`) "None" true)))
          (:`Is Not Valid`
            _))
        (`/Engine/EditorBlueprintResources/StandardMacros.IsValid` (`self.ProjectileMovementRef`)
          (:`Is Valid`
            (`ActorComponent.K2_DestroyComponent` (`self.ProjectileMovementRef`))
            (`PrimitiveComponent.SetCollisionEnabled` (`self.CollisionBox`) "NoCollision")
            (`/Engine/EditorBlueprintResources/StandardMacros.IsValid` _returnvalue
              (:`Is Valid`
                (`self.K2_AttachToComponent` _returnvalue (`.ReturnValue` (`SkinnedMeshComponent.FindClosestBone_K2` _returnvalue _location 0.0 false)) "SnapToTarget" "KeepWorld" "KeepWorld"))
              (:`Is Not Valid`
                (`self.K2_AttachToComponent` _hitcomponent "None" "KeepWorld" "KeepWorld" "KeepWorld")))
            (`GameplayStatics.ApplyDamage` _hitactor (* (`self.ArrowStrength`) 50.0))))))))

(fn `UserConstructionScript`)