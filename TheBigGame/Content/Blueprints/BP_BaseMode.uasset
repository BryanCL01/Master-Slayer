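; BP_BaseMode is a game mode that spawns the player's chosen class and a wave of enemies, then tracks the win condition.
; On BeginPlay it maps the GameInstance's selected class to a character, spawns and possesses it at a PlayerStart.
; It then scatters the GameInstance's enemy count of BP_BaseEnemy at random navigable points around the NavMesh bounds volume.
; EnemyDeafeated decrements the live count and shows the win menu at zero.
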(event `self.ReceiveBeginPlay`
  (bind _asmy_game_instance (cast `/Game/UI/MyGameInstance` (`GameplayStatics.GetGameInstance`)))
  (bind _selectedclass (`/Game/UI/MyGameInstance.SelectedClass` _asmy_game_instance))
  (`KismetSystemLibrary.PrintString` _selectedclass)
  (switch `string` _selectedclass
    (:`Warrior`
      (set `self.ClassToSpawn` "/Game/Blueprints/Characters/BP_WarriorCharacter.BP_WarriorCharacter_C"))
    (:`Wizard`
      (set `self.ClassToSpawn` "/Game/Blueprints/Characters/BP_WizardCharacter.BP_WizardCharacter_C"))
    (:`Rogue`
      (set `self.ClassToSpawn` "/Game/Blueprints/Characters/BP_RogueCharacter.BP_RogueCharacter_C"))
    (:`Marksmen`
      (set `self.ClassToSpawn` "/Game/Blueprints/Characters/BP_MarksmenCharacter.BP_MarksmenCharacter_C")))
  (bind _returnvalue (`GameplayStatics.GetActorOfClass` "/Script/Engine.PlayerStart"))
  (`/Engine/EditorBlueprintResources/StandardMacros.IsValid` _returnvalue
    (:`Is Valid`
      (bind _returnvalue_2 (`|SpawnActorFromClass` (`self.ClassToSpawn`) (`self.GetTransform` _returnvalue) "Undefined" "MultiplyWithRoot" null null))
      (`Controller.Possess` (`GameplayStatics.GetPlayerController` 0) _returnvalue_2)
      (bind _asmy_game_instance_2 (cast `/Game/UI/MyGameInstance` (`GameplayStatics.GetGameInstance`)))
      (bind _returnvalue_3 (`GameplayStatics.GetActorOfClass` "/Script/NavigationSystem.NavMeshBoundsVolume"))
      (bind _output_get (set `self.EnemiesAlive` (`/Game/UI/MyGameInstance.EnemyCount` _asmy_game_instance_2)))
      (for _ (range 1 (+ _output_get 1))
        (bind _randomlocation (`NavigationSystemV1.K2_GetRandomLocationInNavigableRadius` (`self.K2_GetActorLocation` _returnvalue_3) 2000.0 null null))
        (`|SpawnActorFromClass` "/Game/AI/BP_BaseEnemy.BP_BaseEnemy_C" (`KismetMathLibrary.Conv_VectorToTransform` _randomlocation) "AdjustIfPossibleButAlwaysSpawn" "MultiplyWithRoot" null null)))
    (:`Is Not Valid`
      (`KismetSystemLibrary.PrintString` "ERROR: NO PLAYER START FOUND!"))))

(event `EnemyDeafeated`
  (bind _returnvalue (`GameplayStatics.GetPlayerController` 0))
  (bind _output_get (set `self.EnemiesAlive` (- (`self.EnemiesAlive`) 1)))
  (if (<= _output_get 0)
    (bind _returnvalue_2 (`|CreateWidget` "/Game/UI/Win_Menu/WBP_Win_Menu.WBP_Win_Menu_C"))
    (`UserWidget.AddToViewport` _returnvalue_2 0)
    (`WidgetBlueprintLibrary.SetInputMode_UIOnlyEx` _returnvalue null)
    (set `PlayerController.bShowMouseCursor` true _returnvalue)))

(fn `UserConstructionScript`)