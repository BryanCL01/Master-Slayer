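; Base enemy Blueprint with a melee attack, health, a world-space health bar and death handling.
; Attack sphere-traces nearby pawns, damaging the target and playing a montage when it is found.
; Tick updates the health bar and turns it toward the player camera.
; Lethal damage runs once: it stops and unpossesses the AI controller, notifies the game mode, disables capsule collision, plays the death animation, then destroys the actor.
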(event `/Game/AI/BPI_Enemy.Attack`
  (params (TargetActor :type "Actor Object Reference"))
  (bind _returnvalue (`self.K2_GetActorLocation`))
  (bind (_outhits _returnvalue_2) (`KismetSystemLibrary.SphereTraceMultiForObjects` _returnvalue _returnvalue 200.0 (`|MakeArray` "ObjectTypeQuery3" :!type "EObjectTypeQuery Enum")))
  (if _returnvalue_2
    (for _array_element _outhits
      (bind (_bblockinghit _binitialoverlap _time _distance _location _impactpoint _normal _impactnormal _physmat _hitactor) (`GameplayStatics.BreakHitResult` _array_element))
      (if (== TargetActor _hitactor)
        (`GameplayStatics.ApplyDamage` _hitactor 10.0)
        (`|PlayMontage` (`self.Mesh`)
          (:`then`
            (break)))))))

(event `self.ReceiveTick`
  (params (DeltaSeconds :type "Float (single-precision)"))
  (bind _health_bar_widget (`self.Health Bar Widget`))
  ; Health Bar
  (bind _aswp_health_bar (cast `/Game/AI/WP_HealthBar` (`WidgetComponent.GetWidget` (`self.Health Bar Widget`))))
  (`ProgressBar.SetPercent` (`/Game/AI/WP_HealthBar.HealthBar` _aswp_health_bar) (/ (`self.CurrentHealth`) (`self.HealthMax`)))
  (`SceneComponent.K2_SetWorldRotation` _health_bar_widget (`KismetMathLibrary.FindLookAtRotation` (`SceneComponent.K2_GetComponentLocation` _health_bar_widget) (`SceneComponent.K2_GetComponentLocation` (`PlayerCameraManager.TransformComponent` (`GameplayStatics.GetPlayerCameraManager` 0)))) false false))

(event `self.ReceiveAnyDamage`
  (params (Damage :type "Float (single-precision)") (DamageType :type "DamageType Object Reference") (InstigatedBy :type "Controller Object Reference") (DamageCauser :type "Actor Object Reference"))
  (bind _returnvalue (`self.GetController`))
  ; Health Bar
  (bind _output_get (set `self.CurrentHealth` (- (`self.CurrentHealth`) Damage)))
  (if (<= _output_get 0.0)
    (`/Engine/EditorBlueprintResources/StandardMacros.DoOnce` false
      (:`Completed`
        (set `self.IsDead?` true)
        (bind _asbp_aicontroller (cast `/Game/AI/BP_AIController` _returnvalue)
          (:`then`
            (`Controller.StopMovement` _asbp_aicontroller)
            (`Controller.UnPossess` _returnvalue))
          (:`CastFailed`
            _))
        (bind _asbp_base_mode (cast `/Game/Blueprints/BP_BaseMode` (`GameplayStatics.GetGameMode`))
          (:`then`
            (`/Game/Blueprints/BP_BaseMode.EnemyDeafeated` _asbp_base_mode))
          (:`CastFailed`
            _))
        (`PrimitiveComponent.SetCollisionEnabled` (`self.CapsuleComponent`) "NoCollision")
        (`SkeletalMeshComponent.PlayAnimation` (`self.Mesh`) (`self.DeathAnimation`) false)
        (`KismetSystemLibrary.Delay` 3.0)
        (`self.K2_DestroyActor`)))))

(fn `UserConstructionScript`)